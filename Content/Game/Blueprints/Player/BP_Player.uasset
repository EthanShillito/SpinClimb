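; Player Blueprint for a physics-driven character that rolls via input torque and manipulates grabbable objects with the mouse.
; A cursor trace picks up BPI_Grabbable actors with a PhysicsHandle, whose target follows the deprojected mouse each tick, intersected with the player's Y plane.
; Rotate input adjusts the held object's wrapped pitch and prints it.
; Grab, attach and drop actions notify the held actor through messages.
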(event `self.ReceiveTick`
  (params (DeltaSeconds :type "Float (single-precision)"))
  (`self.MoveGrabbed`))

(event `EnhancedInput|/Game/Game/Input/IA_Move`
  (params (ActionValue :type "Float (double-precision)") (ElapsedSeconds :type "Float (double-precision)") (TriggeredSeconds :type "Float (double-precision)") (InputAction :type "InputAction Object Reference" :default "/Game/Game/Input/IA_Move.IA_Move"))
  (:`Triggered`
    (`PrimitiveComponent.AddTorqueInDegrees` (`self.Collision`) (`KismetMathLibrary.MakeVector` 0.0 (* ActionValue (`self.TorqueAmount`))) "None" false)))

(event `EnhancedInput|/Game/Game/Input/IA_Grab`
  (params (ActionValue :type Boolean) (ElapsedSeconds :type "Float (double-precision)") (TriggeredSeconds :type "Float (double-precision)") (InputAction :type "InputAction Object Reference" :default "/Game/Game/Input/IA_Grab.IA_Grab"))
  (bind (_hitresult _returnvalue) (`PlayerController.GetHitResultUnderCursorByChannel` (`GameplayStatics.GetPlayerController` 0) "TraceTypeQuery1" true))
  (bind (_bblockinghit _binitialoverlap _time _distance _location _impactpoint _normal _impactnormal _physmat _hitactor _hitcomponent) (`GameplayStatics.BreakHitResult` _hitresult))
  (:`Started`
    (if (and _returnvalue (`KismetSystemLibrary.DoesImplementInterface` _hitactor "/Game/Game/Blueprints/Grabbable/BPI_Grabbable.BPI_Grabbable_C"))
      (`PhysicsHandleComponent.GrabComponentAtLocationWithRotation` :`self` (`self.PhysicsHandle`) :`Component` _hitcomponent :`Location` _impactpoint)
      (set `self.TargetRotation` 0.0)
      (message `/Game/Game/Blueprints/Grabbable/BPI_Grabbable.PickedUp` _hitactor self)))
  (:`Completed`
    (`self.DropHeldGrabbable`)))

(event `EnhancedInput|/Game/Game/Input/IA_Rotate`
  (params (ActionValue :type "Float (double-precision)") (ElapsedSeconds :type "Float (double-precision)") (TriggeredSeconds :type "Float (double-precision)") (InputAction :type "InputAction Object Reference" :default "/Game/Game/Input/IA_Rotate.IA_Rotate"))
  (bind _returnvalue (`KismetMathLibrary.FWrap` (+ (`self.TargetRotation`) (* ActionValue (`self.GrabbedRotateMultiplier`))) 0.0 360.0))
  (:`Triggered`
    (`KismetSystemLibrary.PrintString` (`KismetStringLibrary.Conv_DoubleToString` _returnvalue))
    (`PhysicsHandleComponent.SetTargetRotation` (`self.PhysicsHandle`) (`KismetMathLibrary.MakeRotator` 0.0 _returnvalue))
    (set `self.TargetRotation` _returnvalue)))

(event `MoveGrabbed`
  (bind (_worldlocation _worlddirection) (`PlayerController.DeprojectMousePositionToWorld` (`GameplayStatics.GetPlayerController` 0)))
  (`PhysicsHandleComponent.SetTargetLocation` (`self.PhysicsHandle`) (+ _worldlocation (* _worlddirection (/ (- (.y (`self.K2_GetActorLocation`)) (.y _worldlocation)) (.y _worlddirection))))))

(event `EnhancedInput|/Game/Game/Input/IA_Attach`
  (params (ActionValue :type Boolean) (ElapsedSeconds :type "Float (double-precision)") (TriggeredSeconds :type "Float (double-precision)") (InputAction :type "InputAction Object Reference" :default "/Game/Game/Input/IA_Attach.IA_Attach"))
  (bind _returnvalue (`PhysicsHandleComponent.GetGrabbedComponent` (`self.PhysicsHandle`)))
  (:`Triggered`
    (`/Engine/EditorBlueprintResources/StandardMacros.IsValid` _returnvalue
      (:`Is Valid`
        (message `/Game/Game/Blueprints/Grabbable/BPI_Grabbable.AttemptAttach` (`ActorComponent.GetOwner` _returnvalue))))))

(event `/Game/Game/Blueprints/Grabbable/BPI_Grabber.DropHeld`
  (`self.DropHeldGrabbable`))

(fn `DropHeldGrabbable`
  (bind _physicshandle (`self.PhysicsHandle`))
  (bind _returnvalue (`PhysicsHandleComponent.GetGrabbedComponent` _physicshandle))
  (`/Engine/EditorBlueprintResources/StandardMacros.IsValid` _returnvalue
    (:`Is Valid`
      (message `/Game/Game/Blueprints/Grabbable/BPI_Grabbable.Dropped` (`ActorComponent.GetOwner` _returnvalue))
      (`PhysicsHandleComponent.ReleaseComponent` _physicshandle))))

(fn `UserConstructionScript`)