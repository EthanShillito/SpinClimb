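; BP_Grabbable is an actor that can be picked up and dropped, and can attach through AttachPointComponents under its Capsule.
; PickedUp stores the Grabber and detaches every attach point, while Dropped clears the Grabber.
; AttemptAttach tries each attach point and, on each success, tells a valid Grabber to release it via DropHeldMessage.
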(event `self.ReceiveBeginPlay`)

(event `/Game/Game/Blueprints/Grabbable/BPI_Grabbable.PickedUp`
  (params (Grabber :type "Object Object Reference"))
  (set `self.Grabber` Grabber)
  (for _array_element (`SceneComponent.GetChildrenComponents` (`self.Capsule`) false)
    (bind _asattach_point_component (cast `AttachPointComponent` _array_element))
    (`AttachPointComponent.bpDetach` _asattach_point_component)))

(event `/Game/Game/Blueprints/Grabbable/BPI_Grabbable.Dropped`
  (set `self.Grabber` null))

(event `/Game/Game/Blueprints/Grabbable/BPI_Grabbable.AttemptAttach`
  (bind _grabber (`self.Grabber`))
  (for _array_element (`SceneComponent.GetChildrenComponents` (`self.Capsule`) false)
    (bind _asattach_point_component (cast `AttachPointComponent` _array_element))
    (bind _returnvalue (`AttachPointComponent.attemptAttach` _asattach_point_component))
    (if _returnvalue
      (`/Engine/EditorBlueprintResources/StandardMacros.IsValid` _grabber
        (:`Is Valid`
          (message `/Game/Game/Blueprints/Grabbable/BPI_Grabber.DropHeld` _grabber))))))

(fn `UserConstructionScript`)